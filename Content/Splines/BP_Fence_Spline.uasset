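; BP_Fence_Spline is a fence actor that lays a chosen static mesh along an editable spline.
; Its construction script adds one deformed spline mesh per segment, using local point locations and tangents, with query and physics collision enabled.
; A Looping flag controls whether an extra segment runs past the last point to close the loop.
; Each segment's end is nudged slightly along local +X; the event graph is unused.
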(fn `UserConstructionScript`
  (for _index (range (+ (- (`SplineComponent.GetNumberOfSplinePoints` (`self.Spline`)) (`KismetMathLibrary.SelectInt` 1 2 (`self.Looping`))) 1))
    (bind _returnvalue (`AddComponent|NODE_AddSplineMeshComponent-0`))
    (bind (_location _tangent) (`SplineComponent.GetLocationAndTangentAtSplinePoint` (`self.Spline`) _index "Local"))
    (bind (_location_2 _tangent_2) (`SplineComponent.GetLocationAndTangentAtSplinePoint` (`self.Spline`) (+ _index 1) "Local"))
    (`SplineMeshComponent.SetStartAndEnd` _returnvalue _location _tangent (`KismetMathLibrary.MakeVector` (- (.x _location_2) -10.0) (.y _location_2) (.z _location_2)) _tangent_2 true)
    (`StaticMeshComponent.SetStaticMesh` _returnvalue (`self.Static Mesh`))
    (`PrimitiveComponent.SetCollisionEnabled` _returnvalue "QueryAndPhysics")))