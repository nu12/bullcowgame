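; Game mode for a Bull Cow game that drives HUD animations on game start, resume, pause and game over.
; GameStart finds and caches the first top-level WBP_HUD, then plays its resume animation.
; A FirstMessage flag makes the first GameResume after start also reveal the top canvas with the clock.
; GameOver passes the win result to the HUD before playing the end animation.
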(event `self.GameStart`
  (bind _wbp_hud (`self.WBP_HUD`))
  (bind _foundwidgets (`WidgetBlueprintLibrary.GetAllWidgetsOfClass` "/Game/UI/WBP_HUD.WBP_HUD_C"))
  (set `self.WBP_HUD` (`|GetArrayItem` _foundwidgets))
  ;[1 1 1] Start Game Animation
  (set `self.FirstMessage` true)
  (`UserWidget.PlayAnimation` _wbp_hud (`/Game/UI/WBP_HUD.GameResumeAnimation` _wbp_hud) 0.0 1 "Forward" 1.0 false))

(event `self.GameResume`
  (bind _wbp_hud (`self.WBP_HUD`))
  (bind _wbp_hud_2 (`self.WBP_HUD`))
  ;[1 1 1] Game Resume & Pause Animations
  (`UserWidget.PlayAnimation` _wbp_hud_2 (`/Game/UI/WBP_HUD.GameResumeAnimation` _wbp_hud_2) 0.0 1 "Forward" 1.0 false)
  ;[1 1 1] Show Clock Animation
  (if (`self.FirstMessage`)
    (`UserWidget.PlayAnimation` _wbp_hud (`/Game/UI/WBP_HUD.ShowTopCanvas` _wbp_hud) 0.0 1 "Forward" 1.0 false)
    (set `self.FirstMessage` false)))

(event `self.GamePause`
  (bind _wbp_hud (`self.WBP_HUD`))
  ;[1 1 1] Game Resume & Pause Animations
  (`UserWidget.PlayAnimation` _wbp_hud (`/Game/UI/WBP_HUD.GamePauseAnimation` _wbp_hud) 0.0 1 "Forward" 1.0 false))

(event `self.GameOver`
  (params (PlayerWon :type Boolean))
  (bind _wbp_hud (`self.WBP_HUD`))
  ;[1 1 1] Game Over Animation
  (set `/Game/UI/WBP_HUD.GameWin` PlayerWon _wbp_hud)
  (`UserWidget.PlayAnimation` _wbp_hud (`/Game/UI/WBP_HUD.GameOverAnimation` _wbp_hud) 0.0 1 "Forward" 1.0 false))

(fn `UserConstructionScript`)